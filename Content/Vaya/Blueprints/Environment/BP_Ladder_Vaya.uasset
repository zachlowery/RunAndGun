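; Ladder actor that lets the player climb, jump off or climb out over the top.
; Entering the trigger disables physics, weapons and most inputs, then aligns the mesh to a helper skeleton.
; Looping timers recheck player state and facing, and query character traces to limit vertical movement or start the timeline-blended top exit.
; Jumping launches the player along an arrow set in construction; ClimbFinishedLogic restores walking, weapons and input.
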(event `Force rotate player left`
  ;[1 1 1] Force rotate player
  (set `/Game/Vaya/Blueprints/Characters/BP_SideScrollerCharacter_Vaya.Player Facing Right?` false (`self.Character object`))
  (`KismetSystemLibrary.K2_UnPauseTimerHandle` (`/Game/Vaya/Blueprints/Characters/BP_SideScrollerCharacter_Vaya.Timer - rotate player left` (`self.Character object`))))

(event `Start climbing logic`
  (bind _returnvalue (`GameplayStatics.GetGameState`))
  (bind _returnvalue_2 (`GameplayStatics.GetGameState`))
  (bind _character_object (`self.Character object`))
  (bind _character_object_2 (`self.Character object`))
  (bind _character_object_3 (`self.Character object`))
  (bind _anim_blueprint (`/Game/SideScrollerKit/Blueprints/BP_Blueprint_Functions.Get player anim blueprint` (`GameplayStatics.GetGameState`)))
  ;[1 1 1] Start climbing logic
  (set `/Game/Vaya/Blueprints/Characters/BP_SideScrollerCharacter_Vaya.Ladder move input open?` true _character_object_3)
  (set `/Game/Vaya/Blueprints/Characters/BP_SideScrollerCharacter_Vaya.Can Leave Ladder From Top` (`self.Can Leave Ladder From Top`) _character_object_3)
  (set `self.Trigger enabled` false)
  (`/Game/Vaya/Blueprints/Characters/BP_SideScrollerCharacter_Vaya.Stop Assault Rifle Shot Loop` (`self.Character object`))
  (set `/Game/SideScrollerKit/Mannequin/Animations/ABP_Mannequin.Is Crouching?` false _anim_blueprint)
  (set `/Game/SideScrollerKit/Mannequin/Animations/ABP_Mannequin.Climbing ladder?` true _anim_blueprint)
  (`/Game/SideScrollerKit/Blueprints/BP_Blueprint_Functions.Set player input` _returnvalue _returnvalue false false true false false false false true)
  (`CharacterMovementComponent.SetMovementMode` (`Character.CharacterMovement` _character_object) "MOVE_None" 0) ; Disabling physics for player so he won't fall
  ;;[1 1 1] Hiding guns with dissolve
  (`/Game/Vaya/Blueprints/Characters/BP_SideScrollerCharacter_Vaya.Start dissolve` _character_object "NewEnumerator0")
  ;;[1 1 1] Hiding Crosshair
  (`/Game/Vaya/Blueprints/Characters/BP_SideScrollerCharacter_Vaya.Hide Crosshair` (`self.Character object`))
  (`KismetSystemLibrary.K2_PauseTimerHandle` (`/Game/Vaya/Blueprints/Characters/BP_SideScrollerCharacter_Vaya.Timer - rotate player left` _character_object_2))
  (`KismetSystemLibrary.K2_PauseTimerHandle` (`/Game/Vaya/Blueprints/Characters/BP_SideScrollerCharacter_Vaya.Timer - rotate player right` _character_object_2))
  ;;[1 1 1] Hiding weapons
  (`/Game/Vaya/Blueprints/Characters/BP_SideScrollerCharacter_Vaya.Change Weapons Visibility` (`self.Character object`) false)
  ;;[1 1 1] Adjusting player rotation to rotation of helper skeleton
  (`SceneComponent.K2_SetWorldRotation` (`Character.Mesh` (`self.Character object`)) (`SceneComponent.K2_GetComponentRotation` (`self.Helper skeletal`)) false true)
  ;;[1 1 1] Disabling inputs
  (`/Game/SideScrollerKit/Blueprints/BP_Blueprint_Functions.Set player input` _returnvalue_2 _returnvalue_2 false false true false false false false true))

(event `Force rotate player right`
  ;[1 1 1] Force rotate player
  (set `/Game/Vaya/Blueprints/Characters/BP_SideScrollerCharacter_Vaya.Player Facing Right?` true)
  (`KismetSystemLibrary.K2_UnPauseTimerHandle` (`/Game/Vaya/Blueprints/Characters/BP_SideScrollerCharacter_Vaya.Timer - rotate player right` (`self.Character object`))))

(event `Timer initials`
  ;[1 1 1] Timer initials
  (bind _returnvalue (`KismetSystemLibrary.K2_SetTimer` null "Ladder use check" 0.01 true))
  (bind _output_get (set `self.Ladder Use Check Handle` _returnvalue))
  (`KismetSystemLibrary.K2_PauseTimerHandle` _output_get)
  (bind _returnvalue_2 (`KismetSystemLibrary.K2_SetTimer` null "Ladder Availability Check" 0.01 true))
  (bind _output_get_2 (set `self.Ladder Availability Check Handle` _returnvalue_2))
  (`KismetSystemLibrary.K2_PauseTimerHandle` _output_get_2))

(event `self.ReceiveBeginPlay`
  ;[1 1 1] Start
  (`self.Timer initials`))

(event `self.Trigger.OnComponentBeginOverlap`
  (params (OverlappedComponent :type "PrimitiveComponent Object Reference") (OtherActor :type "Actor Object Reference") (OtherComp :type "PrimitiveComponent Object Reference") (OtherBodyIndex :type Integer) (bFromSweep :type Boolean) (SweepResult :type "HitResult Structure (by ref)"))
  (bind _character_object (`self.Character object`))
  (bind _character_object_2 (`self.Character object`))
  (bind _character_blueprint (`/Game/SideScrollerKit/Blueprints/BP_Blueprint_Functions.Get player character blueprint` (`GameplayStatics.GetGameState`)))
  (bind _anim_blueprint (`/Game/SideScrollerKit/Blueprints/BP_Blueprint_Functions.Get player anim blueprint` _character_object_2))
  (bind _anim_blueprint_2 (`/Game/SideScrollerKit/Blueprints/BP_Blueprint_Functions.Get player anim blueprint` (`GameplayStatics.GetGameState`)))
  ;[1 1 1] Player enters volume
  (`/Engine/EditorBlueprintResources/StandardMacros.IsValid` _anim_blueprint_2
    (:`Is Valid`
      (if (and (`self.Trigger enabled`) (not (`/Game/SideScrollerKit/Mannequin/Animations/ABP_Mannequin.Climbing ladder?` _anim_blueprint_2)))
        (`/Engine/EditorBlueprintResources/StandardMacros.IsValid` _character_blueprint
          (:`Is Valid`
            (if (and (not (`/Game/SideScrollerKit/Blueprints/BP_SideScrollerCharacter.In Depth Shooting Mode?` _character_blueprint)) (== (`Character.CapsuleComponent` _character_blueprint) OtherComp))
              (bind _character_object_3 (`self.Character object`)
                (:`then`
                  (bind (_relativelocation_x _relativelocation_y _relativelocation_z) (`KismetMathLibrary.BreakVector` (`SceneComponent.RelativeLocation` (`Character.Mesh` _character_object_3))))
                  ;[1 1 1] Checking if players mesh is in default Z location (-95) when starting ladder climb. If not, setting to -95.
                  (if (not (== _relativelocation_z -95.0))
                    (`SceneComponent.K2_SetRelativeLocation` (`Character.Mesh` _character_object_3) (`KismetMathLibrary.MakeVector` _relativelocation_x _relativelocation_y -95.0) false true))
                  (set `/Game/Vaya/Blueprints/Characters/BP_SideScrollerCharacter_Vaya.Normal aiming enabled?` false _character_object_3)
                  (bind _anim_bp_object (`/Game/Vaya/Blueprints/Characters/BP_SideScrollerCharacter_Vaya.Anim BP Object` _character_object_3))
                  (set `/Game/SideScrollerKit/Mannequin/Animations/ABP_Mannequin.Ladder - Finishing Climb` false _anim_bp_object)
                  (set `/Game/SideScrollerKit/Mannequin/Animations/ABP_Mannequin.Ladder move scale` 0.0 _anim_bp_object)
                  (`KismetSystemLibrary.K2_UnPauseTimerHandle` (`self.Ladder Availability Check Handle`))
                  ;[1 1 1] Starting standing check
                  (`KismetSystemLibrary.K2_UnPauseTimerHandle` (`self.Ladder Use Check Handle`))
                  ;[1 1 1] Storing ladder actor reference
                  (set `/Game/Vaya/Blueprints/Characters/BP_SideScrollerCharacter_Vaya.Current Ladder Actor` self (`self.Character object`))
                  (set `/Game/SideScrollerKit/Mannequin/Animations/ABP_Mannequin.Ladder - hitting top` false (`/Game/Vaya/Blueprints/Characters/BP_SideScrollerCharacter_Vaya.Anim BP Object` (`self.Character object`)))
                  ;[1 1 1] Binding jump to let player jump off from ladder
                  (add `/Game/Vaya/Blueprints/Characters/BP_SideScrollerCharacter_Vaya.Player jumped ` (`self.Character object`) (delegate `Player jumped`))
                  ;[1 1 1] Enabling inputs for climbing
                  (`self.State check for ladder`
                    (:`Can use ladder`
                      (`self.Start climbing logic`)
                      (set `/Game/Vaya/Blueprints/Characters/BP_SideScrollerCharacter_Vaya.Ladder move up open?` true (`self.Character object`))
                      (set `/Game/Vaya/Blueprints/Characters/BP_SideScrollerCharacter_Vaya.Ladder move down open?` true _character_object_2)
                      (set `/Game/SideScrollerKit/Mannequin/Animations/ABP_Mannequin.Ladder - hitting floor` false _anim_blueprint)
                      (set `/Game/SideScrollerKit/Mannequin/Animations/ABP_Mannequin.Ladder - hitting top` false _anim_blueprint)
                      ;[1 1 1] Updating player direction
                      (switch `/Game/SideScrollerKit/Blueprints/Enums/E_Right_Left` (`self.Ladder direction`)
                        (:`NewEnumerator2`
                          (set `/Game/Vaya/Blueprints/Characters/BP_SideScrollerCharacter_Vaya.Player Facing Right?` true _character_object))
                        (:`NewEnumerator1`
                          (set `/Game/Vaya/Blueprints/Characters/BP_SideScrollerCharacter_Vaya.Player Facing Right?` false _character_object))))))
                (:`else`)))))))))

(event `Player jumped`
  (bind _returnvalue (`GameplayStatics.GetGameState`))
  (bind _character_object (`self.Character object`))
  (bind _character_object_2 (`self.Character object`))
  (bind _character_object_3 (`self.Character object`))
  (bind _anim_blueprint (`/Game/SideScrollerKit/Blueprints/BP_Blueprint_Functions.Get player anim blueprint` (`GameplayStatics.GetGameState`)))
  (bind _anim_bp_object (`/Game/Vaya/Blueprints/Characters/BP_SideScrollerCharacter_Vaya.Anim BP Object` _character_object_3))
  ;[0.03587 0 0.415] Leaving ladder
  ; Stoping standing check
  ; Player jumped event
  (`KismetSystemLibrary.K2_PauseTimerHandle` (`self.Ladder Use Check Handle`) :!label _label)
  (`KismetSystemLibrary.K2_PauseTimerHandle` (`self.Ladder Availability Check Handle`))
  ;[1 1 1] Player jumped off from ladder
  (set `self.Trigger enabled` true)
  (set `/Game/SideScrollerKit/Mannequin/Animations/ABP_Mannequin.IsInAir?` true _anim_blueprint)
  (set `/Game/SideScrollerKit/Mannequin/Animations/ABP_Mannequin.Jumped from ladder` true _anim_blueprint)
  (`CharacterMovementComponent.SetMovementMode` (`Character.CharacterMovement` (`self.Character object`)) "MOVE_Falling" 0)
  ;;[1 0.04 0.04] Check is player died on ladder
  (if (not (`/Game/Vaya/Blueprints/Characters/BP_SideScrollerCharacter_Vaya.Player Is Dead` (`self.Character object`)))
    ;;[0 0 0] Launching player
    (`Character.LaunchCharacter` (`self.Character object`) (`self.Launch Velocity Direction`) true true))
  (set `/Game/SideScrollerKit/Mannequin/Animations/ABP_Mannequin.Climbing ladder?` false (`/Game/SideScrollerKit/Blueprints/BP_Blueprint_Functions.Get player anim blueprint` (`GameplayStatics.GetGameState`)))
  ;[1 1 1] Unbinding jump when jumped off
  (clear `/Game/Vaya/Blueprints/Characters/BP_SideScrollerCharacter_Vaya.Player jumped ` _character_object_2)
  ;[1 1 1] Update weapons visibility
  (`/Game/Vaya/Blueprints/Characters/BP_SideScrollerCharacter_Vaya.Start dissolve` _character_object_2 "NewEnumerator0")
  (`/Game/Vaya/Blueprints/Characters/BP_SideScrollerCharacter_Vaya.Change Weapons Visibility` _character_object_2 false)
  (`/Game/Vaya/Blueprints/Characters/BP_SideScrollerCharacter_Vaya.Update current weapon` _character_object_2)
  ;[1 1 1] Showing Crosshair
  (`/Game/Vaya/Blueprints/Characters/BP_SideScrollerCharacter_Vaya.Show Crosshair` (`self.Character object`))
  ;[1 1 1] Rotating player in opposite direction from ladder when he jumped off
  (switch `/Game/SideScrollerKit/Blueprints/Enums/E_Right_Left` (`self.Ladder direction`)
    (:`NewEnumerator2`
      (set `/Game/Vaya/Blueprints/Characters/BP_SideScrollerCharacter_Vaya.Player Facing Right?` false)
      (`/Game/Vaya/Blueprints/Characters/BP_SideScrollerCharacter_Vaya.Reset facing left` _character_object_3)
      (`/Game/Vaya/Blueprints/Characters/BP_SideScrollerCharacter_Vaya.Reset facing right` _character_object_3)
      (set `/Game/SideScrollerKit/Mannequin/Animations/ABP_Mannequin.Player Facing Right? (Anim BP)` false _anim_bp_object)
      (`KismetSystemLibrary.K2_UnPauseTimerHandle` (`/Game/Vaya/Blueprints/Characters/BP_SideScrollerCharacter_Vaya.Timer - rotate player left` _character_object)))
    (:`NewEnumerator1`
      (set `/Game/Vaya/Blueprints/Characters/BP_SideScrollerCharacter_Vaya.Player Facing Right?` true _character_object_3)
      (`/Game/Vaya/Blueprints/Characters/BP_SideScrollerCharacter_Vaya.Reset facing left`)
      (`/Game/Vaya/Blueprints/Characters/BP_SideScrollerCharacter_Vaya.Reset facing right`)
      (set `/Game/SideScrollerKit/Mannequin/Animations/ABP_Mannequin.Player Facing Right? (Anim BP)` true _anim_bp_object)
      (`KismetSystemLibrary.K2_UnPauseTimerHandle` (`/Game/Vaya/Blueprints/Characters/BP_SideScrollerCharacter_Vaya.Timer - rotate player right` _character_object))))
  ;[1 1 1] Enabling player inputs
  (`/Game/SideScrollerKit/Blueprints/BP_Blueprint_Functions.Set player input` _returnvalue _returnvalue)
  ;;[0 0 0] Making sure that player anim state won't go into jump end or run right after jump off ladder
  (`KismetSystemLibrary.Delay` 0.2)
  (set `/Game/SideScrollerKit/Mannequin/Animations/ABP_Mannequin.Jumped from ladder` false (`/Game/SideScrollerKit/Blueprints/BP_Blueprint_Functions.Get player anim blueprint` (`GameplayStatics.GetGameState`)))
  (set `/Game/Vaya/Blueprints/Characters/BP_SideScrollerCharacter_Vaya.Depth Aiming Input Open?` true (`self.Character object`))
  (`KismetSystemLibrary.Delay` 0.4)
  (set `/Game/Vaya/Blueprints/Characters/BP_SideScrollerCharacter_Vaya.Normal aiming enabled?` true (`self.Character object`)))

(event `self.Trigger.OnComponentEndOverlap`
  (params (OverlappedComponent :type "PrimitiveComponent Object Reference") (OtherActor :type "Actor Object Reference") (OtherComp :type "PrimitiveComponent Object Reference") (OtherBodyIndex :type Integer))
  (bind _character_object (`self.Character object`))
  (bind _character_blueprint (`/Game/SideScrollerKit/Blueprints/BP_Blueprint_Functions.Get player character blueprint` (`GameplayStatics.GetGameState`)))
  ;[1 1 1] Player left volume
  (`/Engine/EditorBlueprintResources/StandardMacros.IsValid` _character_blueprint
    (:`Is Valid`
      (if (and (== (`Character.CapsuleComponent` _character_blueprint) OtherComp) (`KismetSystemLibrary.IsValid` _character_blueprint))
        (if (not (`/Game/SideScrollerKit/Mannequin/Animations/ABP_Mannequin.Climbing ladder?` (`/Game/SideScrollerKit/Blueprints/BP_Blueprint_Functions.Get player anim blueprint` (`GameplayStatics.GetGameState`))))
          ;;[1 1 1] Stoping standing check
          (`KismetSystemLibrary.K2_PauseTimerHandle` (`self.Ladder Use Check Handle`))
          (set `self.Trigger enabled` true)
          ;[1 1 1] Unbinding jump
          (clear `/Game/Vaya/Blueprints/Characters/BP_SideScrollerCharacter_Vaya.Player jumped ` (`self.Character object`))
          ;[1 0.04 0.04] Check is player died on ladder
          (if (`/Game/Vaya/Blueprints/Characters/BP_SideScrollerCharacter_Vaya.Player Is Dead` _character_object)
            (`/Game/Vaya/Blueprints/Characters/BP_SideScrollerCharacter_Vaya.Update current weapon` _character_object)
            (goto _label)))))))

(event `Ladder use check`
  (bind _player_facing_right_ (`/Game/Vaya/Blueprints/Characters/BP_SideScrollerCharacter_Vaya.Player Facing Right?` (`self.Character object`)))
  ;[1 1 1] Checking if player can use ladder.
  (`self.State check for ladder`
    (:`Can use ladder`
      (set `self.Trigger enabled` true)
      ;[1 1 1] Making sure that player is rotated towards ladder. In some cases player could rotate opposite right before grabing ladder and that couse a bug.
      (switch `/Game/SideScrollerKit/Blueprints/Enums/E_Right_Left` (`self.Ladder direction`)
        (:`NewEnumerator2`
          (if _player_facing_right_
            ;[1 1 1] Checking if crosshair is not visible
            (`self.Update crosshair visibility` :!label _label_2)
            (else
              (`self.Rotate player towards ladder` :!label _label_3))))
        (:`NewEnumerator1`
          (if _player_facing_right_
            (goto _label_3)
            (else
              (goto _label_2))))))
    (:`Can't use ladder`
      (set `self.Trigger enabled` false))))

(event `Climb Top Logic`
  (bind _character_object (`self.Character object`))
  (bind _anim_bp_object (`/Game/Vaya/Blueprints/Characters/BP_SideScrollerCharacter_Vaya.Anim BP Object` _character_object))
  ;[1 1 1] Starting climb on top logic
  (set `/Game/SideScrollerKit/Mannequin/Animations/ABP_Mannequin.Is Crouching?` true _anim_bp_object)
  (set `/Game/SideScrollerKit/Mannequin/Animations/ABP_Mannequin.Ladder - Finishing Climb` true _anim_bp_object)
  (set `/Game/Vaya/Blueprints/Characters/BP_SideScrollerCharacter_Vaya.Ladder move input open?` false _character_object)
  (set `/Game/Vaya/Blueprints/Characters/BP_SideScrollerCharacter_Vaya.Jump Input Open?` false _character_object)
  (set `/Game/Vaya/Blueprints/Characters/BP_SideScrollerCharacter_Vaya.Ladder move down open?` false _character_object)
  (set `/Game/Vaya/Blueprints/Characters/BP_SideScrollerCharacter_Vaya.Ladder move up open?` false _character_object)
  (`CharacterMovementComponent.SetMovementMode` (`Character.CharacterMovement` _character_object) "MOVE_Flying" 0) ; Disabling physics for player so he won't fall
  (`TimelineComponent.SetPlayRate` (`self.Finishing animation blend `) 1.3)
  (bind (_direction _alpha _mesh_location_z) (`Timeline|Finishing animation blend` :!via `PlayFromStart`)
    (:`Update`
      (set `/Game/SideScrollerKit/Mannequin/Animations/ABP_Mannequin.Ladder Climb Top Alpha Blend` _alpha (`/Game/Vaya/Blueprints/Characters/BP_SideScrollerCharacter_Vaya.Anim BP Object` (`self.Character object`)))
      (if (`/Game/SideScrollerKit/Mannequin/Animations/ABP_Mannequin.Is Crouching?` null)
        (`SceneComponent.K2_SetRelativeLocation` (`Character.Mesh` (`self.Character object`)) (`KismetMathLibrary.MakeVector` 0.0 0.0 _mesh_location_z) false true)))))

(fn `Climb Finished Logic`
  (bind _returnvalue (`GameplayStatics.GetGameState`))
  (bind (_character_object _character_object_2) (`self.Character object`))
  (bind (_character_object_3 _character_object_4) (`self.Character object`))
  (bind (_character_object_5 _character_object_6) (`self.Character object`))
  (bind _anim_bp_object (`/Game/SideScrollerKit/Blueprints/BP_SideScrollerCharacter.Anim BP Object` _character_object_2))
  ;[0.03587 0 0.415] Leaving ladder - player finished climbing
  (`KismetSystemLibrary.K2_PauseTimerHandle` (`self.Ladder Use Check Handle`))
  (`/Game/SideScrollerKit/Blueprints/BP_SideScrollerCharacter.Start stand up check` (`.Character object` (`self.Character object`)))
  ;[1 1 1] Player jumped off from ladder
  (set `self.Trigger enabled` true)
  (`CharacterMovementComponent.SetMovementMode` (`Character.CharacterMovement` (`.Character object` (`self.Character object`))) "MOVE_Walking" 0)
  ;[1 1 1] Unbinding jump when jumped off
  (clear `/Game/SideScrollerKit/Blueprints/BP_SideScrollerCharacter.Player jumped ` _character_object_4)
  ;[1 1 1] Showing current selected weapon
  (`/Game/SideScrollerKit/Blueprints/BP_SideScrollerCharacter.Update current weapon` _character_object_4)
  ;[1 1 1] Showing Crosshair
  (`/Game/SideScrollerKit/Blueprints/BP_SideScrollerCharacter.Show Crosshair` (`.Character object` (`self.Character object`)))
  ;[0 0 0] Unhiding guns with dissolve
  (`/Game/SideScrollerKit/Blueprints/BP_SideScrollerCharacter.Start dissolve` (`.Character object` (`self.Character object`)) "NewEnumerator4")
  (`/Game/SideScrollerKit/Blueprints/BP_SideScrollerCharacter.Change Weapons Visibility` _character_object_6 true)
  ;[1 1 1] Showing current selected weapon
  (`/Game/SideScrollerKit/Blueprints/BP_SideScrollerCharacter.Update current weapon` _character_object_6)
  ;[1 1 1] Enabling player inputs
  (`/Game/SideScrollerKit/Blueprints/BP_Blueprint_Functions.Set player input` _returnvalue _returnvalue)
  (set `/Game/SideScrollerKit/Blueprints/BP_SideScrollerCharacter.Depth Aiming Input Open?` true (`.Character object` (`self.Character object`)))
  (set `/Game/SideScrollerKit/Blueprints/BP_SideScrollerCharacter.Normal aiming enabled?` true _character_object_2)
  ;[1 1 1] Reseting aiming rotation
  (switch `/Game/SideScrollerKit/Blueprints/Enums/E_Right_Left` (`self.Ladder direction`)
    (:`NewEnumerator2`
      (`/Game/SideScrollerKit/Blueprints/BP_SideScrollerCharacter.Reset facing left` _character_object_2))
    (:`NewEnumerator1`
      (`/Game/SideScrollerKit/Blueprints/BP_SideScrollerCharacter.Reset facing right` _character_object_2)))
  (set `/Game/SideScrollerKit/Mannequin/Animations/ABP_Mannequin.Ladder - Finishing Climb` false _anim_bp_object)
  ;[1 1 1] Setting crouch walk speed when player is crouching right after climbing.
  (if (`/Game/SideScrollerKit/Mannequin/Animations/ABP_Mannequin.Is Crouching?` _anim_bp_object)
    (set `CharacterMovementComponent.MaxWalkSpeed` (`/Game/SideScrollerKit/Blueprints/BP_SideScrollerCharacter.Crouch walk speed` _character_object_2) (`Character.CharacterMovement` _character_object_2)))
  (return))

(fn `Ladder Availability Check`
  (bind (_character_object _character_object_2) (`self.Character object`))
  (bind _anim_blueprint (`/Game/SideScrollerKit/Blueprints/BP_Blueprint_Functions.Get player anim blueprint` (`GameplayStatics.GetGameState`)))
  (bind _anim_blueprint_2 (`/Game/SideScrollerKit/Blueprints/BP_Blueprint_Functions.Get player anim blueprint` (`GameplayStatics.GetGameState`)))
  ;[1 1 1] Fireing line trace to look for ladder back wall
  (bind (_character_object_3 _character_object_4) (`self.Character object`)
    (:`then`
      (bind (_trace_up_hit_ _trace_down_hit_) (`/Game/SideScrollerKit/Blueprints/BP_SideScrollerCharacter.Ladder Availability Check` _character_object_4 (`self.Ladder direction`)))
      ;[1 1 1] Top trace
      (if _trace_up_hit_
        (set `/Game/SideScrollerKit/Blueprints/BP_SideScrollerCharacter.Ladder move up open?` true _character_object_2)
        (set `/Game/SideScrollerKit/Mannequin/Animations/ABP_Mannequin.Ladder - hitting top` false _anim_blueprint)
        (else
          (set `/Game/SideScrollerKit/Blueprints/BP_SideScrollerCharacter.Ladder move up open?` false _character_object_2)
          (set `/Game/SideScrollerKit/Mannequin/Animations/ABP_Mannequin.Ladder - hitting top` true _anim_blueprint)
          (if (`self.Can Leave Ladder From Top`)
            ;[1 1 1] Starting climb finish logic
            (`KismetSystemLibrary.K2_PauseTimerHandle` (`self.Ladder Availability Check Handle`))
            (`self.Climb Top Logic`)
            (return)
            (else
              _))))
      ;[1 1 1] Down trace
      (if _trace_down_hit_
        (set `/Game/SideScrollerKit/Blueprints/BP_SideScrollerCharacter.Ladder move down open?` true (`.Character object` (`self.Character object`)))
        (set `/Game/SideScrollerKit/Mannequin/Animations/ABP_Mannequin.Ladder - hitting floor` false _anim_blueprint_2)
        (else
          (set `/Game/SideScrollerKit/Blueprints/BP_SideScrollerCharacter.Ladder move down open?` false (`.Character object` (`self.Character object`)))
          (set `/Game/SideScrollerKit/Mannequin/Animations/ABP_Mannequin.Ladder - hitting floor` true _anim_blueprint_2)))
      (return))
    (:`else`
      (return))))

(fn `Rotate player towards ladder`
  ;[0 0.05677 0.22] Making sure character is rotated towards ladder
  (switch `/Game/SideScrollerKit/Blueprints/Enums/E_Right_Left` (`self.Ladder direction`)
    (:`NewEnumerator2`
      (if (not (!= (`SceneComponent.K2_GetComponentRotation` (`Character.Mesh` (`.Character object` (`self.Character object`)))) (`SceneComponent.K2_GetComponentRotation` (`self.Helper skeletal`))))
        (`self.Force rotate player right`)))
    (:`NewEnumerator1`
      (if (not (!= (`SceneComponent.K2_GetComponentRotation` (`Character.Mesh` (`.Character object` (`self.Character object`)))) (`SceneComponent.K2_GetComponentRotation` (`self.Helper skeletal`))))
        (`self.Force rotate player left`))))
  ;;[1 1 1] Hiding Crosshair
  (`/Game/SideScrollerKit/Blueprints/BP_SideScrollerCharacter.Hide Crosshair` (`.Character object` (`self.Character object`)))
  (return))

(fn `Update crosshair visibility`
  (bind (_character_object _character_object_2) (`self.Character object`))
  ;[1 1 1] Update crosshair visibility
  (if (`SceneComponent.IsVisible` (`/Game/SideScrollerKit/Blueprints/BP_Crosshair_3D.Crosshair Material Billboard` (`/Game/SideScrollerKit/Blueprints/BP_SideScrollerCharacter.Crosshair Widget` _character_object_2)))
    (`/Game/SideScrollerKit/Blueprints/BP_SideScrollerCharacter.Hide Crosshair` _character_object_2))
  (return))

(fn `UserConstructionScript`
  (bind _jump_launch_direction_arrow (`self.Jump Launch Direction Arrow`))
  (`SceneComponent.K2_SetRelativeLocation` (`self.Trigger`) (`self.Trigger location`) false false)
  (`BoxComponent.SetBoxExtent` (`self.Trigger`) (`self.Trigger extents`) true)
  (`SceneComponent.K2_SetRelativeRotation` _jump_launch_direction_arrow (`self.Jump Off Launch Direction`) false false)
  (set `self.Launch Velocity Direction` (* (`SceneComponent.GetForwardVector` _jump_launch_direction_arrow) (`self.Jump Off Launch Power`))))